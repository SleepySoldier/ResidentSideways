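; BP_PickupActor is a world item pickup that shows the mesh from its item info and adds that item to an interacting actor's inventory.
; The construction script sets the mesh, and highlight events toggle an interactable overlay material on it.
; On interact it calls AddItem on the actor's BPC_Inventory with the item and amount.
; If that succeeds, it destroys itself and re-enables the interacting character's input.
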(event `/Game/_Project/Blueprint/Definitions/Interface/BPI_Interact.OnHighlight`
  (`MeshComponent.SetOverlayMaterial` (`self.StaticMesh`) "/Game/_Project/Materials/Outline/MI_Interactable.MI_Interactable"))

(event `/Game/_Project/Blueprint/Definitions/Interface/BPI_Interact.OnUnhighlight`
  (`MeshComponent.SetOverlayMaterial` (`self.StaticMesh`) null))

(event `/Game/_Project/Blueprint/Definitions/Interface/BPI_Interact.OnInteract`
  (params (InteractingActor :type "Actor Object Reference"))
  (set `self.Interacting Actor` InteractingActor)
  (bind _returnvalue (`InventoryComponent.AddItem` (`self.GetComponentByClass` InteractingActor "/Game/_Project/Blueprint/Inventory/BPC_Inventory.BPC_Inventory_C") (`self.ItemInfo`) (`self.Amount`)))
  (if _returnvalue
    (`self.K2_DestroyActor`)
    (`self.EnableInput` (`self.Interacting Actor`) (cast `PlayerController` (`Pawn.GetController` (cast `Character` (`self.Interacting Actor`) :!pure true)) :!pure true))))

(fn `UserConstructionScript`
  (`StaticMeshComponent.SetStaticMesh` (`self.StaticMesh`) (`ItemInfoAsset.PickupMesh` (`self.ItemInfo`))))