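; BP_Bandaid is an inventory item that heals the actor that uses it.
; Its UseItem event reads that actor's max HP through an interface message and sends back a heal message for that value scaled by the item's RestoreAmount.
; It then removes one unit at the given slot index from the user's BPC_Inventory component.
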(event `self.UseItem`
  (params (Actor :type "Actor Object Reference") (Index :type Integer))
  (set `self.Item Index` Index)
  (bind _output_get (set `self.Use Actor` Actor))
  (bind _maxhp (message `/Game/_Project/Blueprint/Definitions/Interface/BPI_Damage.GetMaxHp` _output_get))
  (message `/Game/_Project/Blueprint/Definitions/Interface/BPI_Damage.Heal` _output_get (* _maxhp (`ItemInfoAsset.RestoreAmount` (`self.ItemInfo`))))
  (`/Game/_Project/Blueprint/Inventory/BPC_Inventory.RemoveItem` (`Actor.GetComponentByClass` (`self.Use Actor`) "/Game/_Project/Blueprint/Inventory/BPC_Inventory.BPC_Inventory_C") (`self.Item Index`) 1))