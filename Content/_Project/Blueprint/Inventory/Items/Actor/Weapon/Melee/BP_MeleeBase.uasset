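; Base Blueprint for melee weapon items that plays combo attacks on the owner's skeletal mesh.
; UseWeapon locks move input and plays the attack montage from WeaponInfo, starting at the section indexed by ComboCounter.
; Montage notifies drive the combo: Combo Start permits another attack and advances the counter, while Combo End resets it.
; Blend out also resets the combo and restores movement, whereas interruption only restores movement.
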(event `self.UseWeapon`
  (params (UsingActor :type "Actor Object Reference"))
  (bind ((`ActorAttackAnim` _actorattackanim)) (break `WeaponInfo` (`ItemInfoAsset.WeaponInfo` (`self.WeaponInfo`))))
  (if (or (not (`self.IsAttacking`)) (`self.CanAttackAgain`))
    (`Controller.SetIgnoreMoveInput` (`/Game/_Project/Blueprint/Definitions/FunctionLibrary/BFL_HandyTools.GetLocalPlayerController` (`self.GetOwner`)) true)
    (set `self.IsAttacking` true)
    (bind _notifyname (`|PlayMontage` (`self.GetComponentByClass` (`self.GetOwner`) "/Script/Engine.SkeletalMeshComponent") _actorattackanim 1.0 0.0 (`AnimMontage.GetSectionName` _actorattackanim (`self.ComboCounter`)))
      (:`OnBlendOut`
        (`self.EndAttack`))
      (:`OnInterrupted`
        (`Controller.SetIgnoreMoveInput` (`/Game/_Project/Blueprint/Definitions/FunctionLibrary/BFL_HandyTools.GetLocalPlayerController` (`self.GetOwner`)) false))
      (:`OnNotifyBegin`
        (switch `name` _notifyname
          (:`ComboStart`
            (set `self.CanAttackAgain` true)
            (`/Engine/EditorBlueprintResources/StandardMacros.IncrementInt` (`self.ComboCounter`)))
          (:`ComboEnd`
            (`self.EndAttack`)))))))

(event `EndAttack`
  (set `self.CanAttackAgain` false)
  (set `self.ComboCounter` 0)
  (set `self.IsAttacking` false)
  (`Controller.SetIgnoreMoveInput` (`/Game/_Project/Blueprint/Definitions/FunctionLibrary/BFL_HandyTools.GetLocalPlayerController` (`self.GetOwner`)) false))

(fn `UserConstructionScript`
  (`parent.UserConstructionScript`))