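; Base firearm Blueprint that handles firing and reloading for ranged weapons, driven by WeaponInfo.
; UseWeapon runs semi-auto, looping-timer full-auto or three-shot burst, all feeding OnFire, which plays animations and decrements the inventory slot's round count.
; Shots resolve as hitscan, cone spread or spawned BP_Projectile, with impacts sending randomized damage through HandleImpact.
; Reload checks and draws ammo through the owner's BPC_Inventory, updating the magazine on a montage notify.
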(event `self.ReceiveBeginPlay`
  (`parent.ReceiveBeginPlay`))

(event `self.UseWeapon`
  (if (not (`self.IsFiring`))
    (if (not (`self.MagEmpty`))
      (set `self.IsFiring` true)
      (switch `EWeaponFireMode` (`.FireMode` (break `WeaponInfo` (`ItemInfoAsset.WeaponInfo` (`self.WeaponInfo`))))
        (:`SemiAuto`
          (`self.SemiAutoFire`))
        (:`FullAuto`
          (`self.FullAutoFire`))
        (:`BurstFire`
          (`self.BurstFire`)))
      (else
        (`GameplayStatics.PlaySound2D` "/Game/_WeaponsPacks/MilitaryWeapDark/Sound/Pistol/Pistol_MagEject_Cue.Pistol_MagEject_Cue" 1.0 1.0 0.0 null null)))))

(event `SemiAutoFire`
  (`self.OnFire`)
  (`KismetSystemLibrary.Delay` (`.FireRate` (break `WeaponInfo` (`ItemInfoAsset.WeaponInfo` (`self.WeaponInfo`)))))
  (set `self.IsFiring` false))

(event `FullAutoFire`
  (bind ((`FireRate` _firerate)) (break `WeaponInfo` (`ItemInfoAsset.WeaponInfo` (`self.WeaponInfo`))))
  ;[0 0 0 0.5] Full Auto fire
  (set `self.CanFireAgain` true)
  (bind _returnvalue (`KismetSystemLibrary.K2_SetTimerDelegate` (delegate `StartFullAutoFire`) _firerate true false (* _firerate -1.0)))
  (set `self.FullAutoTimerHandle` _returnvalue))

(event `StartFullAutoFire`
  ;[0 0 0 0.5] Full Auto fire
  (if (and (`self.CanFireAgain`) (not (`self.MagEmpty`)))
    (`self.OnFire`)
    (else
      (`self.EndFullAuto`))))

(event `BurstFire`
  (bind ((`FireRate` _firerate)) (break `WeaponInfo` (`ItemInfoAsset.WeaponInfo` (`self.WeaponInfo`))))
  ;[0 0 0 0.5] Burst Fire
  (bind _returnvalue (`KismetSystemLibrary.K2_SetTimerDelegate` (delegate `BurstFireStart`) _firerate true false (* _firerate -1.0)))
  (set `self.BurstFireTimerHandle` _returnvalue))

(event `BurstFireStart`
  ;[0 0 0 0.5] Burst Fire
  (if (or (== (`self.BurstCounteer`) 3) (`self.MagEmpty`))
    (`KismetSystemLibrary.K2_ClearAndInvalidateTimerHandle` (`self.BurstFireTimerHandle`))
    (set `self.IsFiring` false)
    (set `self.BurstCounteer` 0)
    (else
      (`/Engine/EditorBlueprintResources/StandardMacros.IncrementInt` (`self.BurstCounteer`)
        (:`  `
          (`self.OnFire`))))))

(event `OnFire`
  (bind (_socketlocation _socketforwardvector) (`self.GetLineTraceStartEnd`))
  (bind (_socketlocation_2 _socketforwardvector_2) (`self.GetLineTraceStartEnd`))
  (bind (_socketlocation_3 _socketforwardvector_3) (`self.GetLineTraceStartEnd`))
  (bind ((`WeaponAttackAnim` _weaponattackanim) (`ActorAttackAnim` _actorattackanim)) (break `WeaponInfo` (`ItemInfoAsset.WeaponInfo` (`self.WeaponInfo`))))
  (bind _output (`|GetArrayItem` (`InventoryComponent.Inventory` (`self.GetOwnerInventory`)) (`self.WeaponItemIndex`)))
  (bind _returnvalue (- (`.AmountHeld` (break `ItemSlotInfo` _output)) 1))
  ; OnFire
  (`SkeletalMeshComponent.PlayAnimation` (`self.SkeletalMesh`) _weaponattackanim false)
  (`|PlayMontage` (`self.GetComponentByClass` (`self.GetOwner`) "/Script/Engine.SkeletalMeshComponent") _actorattackanim
    (:`then`
      (setmembers `ItemSlotInfo` :`StructRef` _output :`AmountHeld` _returnvalue)
      (if (<= _returnvalue 0)
        (set `self.MagEmpty` true)
        (else
          (set `self.MagEmpty` false)))
      (switch `EWeaponFireType` (`.FireType` (break `WeaponInfo` (`ItemInfoAsset.WeaponInfo` (`self.WeaponInfo`))))
        (:`HitScan`
          (`self.HitscanDamage` _socketlocation_2 (+ _socketlocation_2 (* _socketforwardvector_2 (`self.HitscanFireRange`)))))
        (:`Spread`
          (for _ (range 1 (+ (`self.SpreadProjectileAmount`) 1))
            (`self.HitscanDamage` _socketlocation_3 (+ _socketlocation_3 (* (`KismetMathLibrary.RandomUnitVectorInConeInDegrees` _socketforwardvector_3 15.0) (`self.HitscanFireRange`))))))
        (:`Projectile`
          (bind _returnvalue_2 (`|SpawnActorFromClass` "/Game/_Project/Blueprint/Inventory/Items/Actor/Weapon/Ranged/Projectile/BP_Projectile.BP_Projectile_C" (`KismetMathLibrary.MakeTransform` _socketlocation (`KismetMathLibrary.FindLookAtRotation` _socketlocation (+ _socketlocation _socketforwardvector))) "AlwaysSpawn" "MultiplyWithRoot" (`self.GetOwner`) null))
          (`/Engine/EditorBlueprintResources/StandardMacros.IsValid` _returnvalue_2
            (:`Is Valid`
              (add `/Game/_Project/Blueprint/Inventory/Items/Actor/Weapon/Ranged/Projectile/BP_Projectile.OnImpacts` _returnvalue_2 (`|CreateDelegate` :!event `HandleImpact`)))))))))

(event `HandleImpact`
  (params (Hit :type "HitResult Structure"))
  (bind (_bblockinghit _binitialoverlap _time _distance _location _impactpoint _normal _impactnormal _physmat _hitactor) (`GameplayStatics.BreakHitResult` Hit))
  (bind ((`BasePower` _basepower)) (break `WeaponInfo` (`ItemInfoAsset.WeaponInfo` (`self.WeaponInfo`))))
  ; OnFire
  ;; Deal damage
  (message `/Game/_Project/Blueprint/Definitions/Interface/BPI_Damage.TakeDamage` _hitactor (make `/Game/_Project/Blueprint/Definitions/Stuct/Damage/F_Damageinfo` (`KismetMathLibrary.RandomFloatInRange` (* _basepower 0.8) (* _basepower 1.2)) _impactpoint "NewEnumerator1" (`self.GetOwner`))))

(event `self.ReloadFirearm`
  (bind _returnvalue (`self.GetOwnerInventory`))
  (bind (_output_item _output_amountheld) (break `ItemSlotInfo` (`|GetArrayItem` (`InventoryComponent.Inventory` _returnvalue) (`self.WeaponItemIndex`))))
  (if (`self.CheckCanReload`)
    (bind _notifyname (`|PlayMontage` (`self.GetComponentByClass` (`self.GetOwner`) "/Script/Engine.SkeletalMeshComponent") (`.ActorReloadAnim` (break `WeaponInfo` (`ItemInfoAsset.WeaponInfo` (`self.WeaponInfo`)))))
      (:`then`
        (set `self.IsReloading` true))
      (:`OnNotifyBegin`
        (switch `name` _notifyname
          (:`Reload`
            (bind _newroundsinmag (`/Game/_Project/Blueprint/Inventory/BPC_Inventory.DoReload` _returnvalue _output_amountheld (`self.WeaponInfo`)))
            (setmembers `ItemSlotInfo` :`StructRef` (`|GetArrayItem` (`InventoryComponent.Inventory` (`self.GetOwnerInventory`)) (`self.WeaponItemIndex`)) :`AmountHeld` _newroundsinmag)
            (set `self.IsReloading` false)
            (set `self.MagEmpty` false)))))))

(event `self.EndUseWeapon`
  (`self.EndFullAuto`))

(fn `CheckCanReload`
  (returns (ReturnValue :type Boolean))
  (bind ((`MaxMagCapacity` _maxmagcapacity) (`FireType` _firetype) (`FirearmAmmoTag` _firearmammotag)) (break `WeaponInfo` (`ItemInfoAsset.WeaponInfo` (`self.WeaponInfo`))))
  (bind (_output_item _output_amountheld) (break `ItemSlotInfo` (`|GetArrayItem` (`InventoryComponent.Inventory` (`self.GetOwnerInventory`)) (`self.WeaponItemIndex`))))
  (return (and (< _output_amountheld (`.MaxMagCapacity` (break `WeaponInfo` (`ItemInfoAsset.WeaponInfo` (`self.WeaponInfo`))))) (not (`self.IsReloading`)) (> (`/Game/_Project/Blueprint/Inventory/BPC_Inventory.DoesHaveAmmo` (`self.GetOwnerInventory`) _firearmammotag) _maxmagcapacity))))

(fn `EndFullAuto`
  (`KismetSystemLibrary.K2_ClearAndInvalidateTimerHandle` (`self.FullAutoTimerHandle`))
  (set `self.IsFiring` false))

(fn `GetOwnerInventory`
  (returns (ReturnValue :type "/Game/_Project/Blueprint/Inventory/BPC_Inventory Object Reference"))
  (return (`self.GetComponentByClass` (`self.GetOwner`) "/Game/_Project/Blueprint/Inventory/BPC_Inventory.BPC_Inventory_C")))

(fn `HitscanDamage`
  (params (Start :type "Vector Structure") (End :type "Vector Structure"))
  (bind _outhit (`KismetSystemLibrary.LineTraceSingleForObjects` Start End (`|MakeArray` "ObjectTypeQuery3" :!type "EObjectTypeQuery Enum") false (`|MakeArray` (`self.GetOwner`))))
  (`self.HandleImpact` _outhit))

(fn `UserConstructionScript`
  (`parent.UserConstructionScript`))