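; BP_Projectile is a weapon projectile that reacts when its overlap sphere touches any actor other than its owner.
; On overlap, it runs a stationary Pawn-only sphere trace of the same radius to obtain a hit result, without checking that the trace succeeded.
; That hit drives a Niagara impact effect selected by surface type and the OnImpacts dispatcher, then the projectile destroys itself.
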(event `self.OverlapSphere.OnComponentBeginOverlap`
  (params (OverlappedComponent :type "PrimitiveComponent Object Reference") (OtherActor :type "Actor Object Reference") (OtherComp :type "PrimitiveComponent Object Reference") (OtherBodyIndex :type Integer) (bFromSweep :type Boolean) (SweepResult :type "HitResult Structure (by ref)"))
  (bind _returnvalue (`self.K2_GetActorLocation`))
  (if (!= OtherActor (`self.GetOwner`))
    (bind _outhit (`KismetSystemLibrary.SphereTraceSingleForObjects` _returnvalue _returnvalue (`SphereComponent.SphereRadius` (`self.OverlapSphere`)) (`|MakeArray` "ObjectTypeQuery3" :!type "EObjectTypeQuery Enum")))
    (`self.ImpactFX` _outhit)
    (`self.OnImpacts` _outhit)
    (`self.K2_DestroyActor`)))

(event `self.ImpactFX`
  (params (HitInfo :type "HitResult Structure"))
  (`NiagaraFunctionLibrary.SpawnSystemAtLocation` (select `EPhysicalSurface` (`GameplayStatics.GetSurfaceType` HitInfo) :`SurfaceType_Default` "/Game/ParticleFX/BloodPack/Hit/Niagara/NS_BulletHit_Med.NS_BulletHit_Med" :!type "NiagaraSystem Object Reference") (`.Location` (`GameplayStatics.BreakHitResult` HitInfo))))

(fn `UserConstructionScript`)