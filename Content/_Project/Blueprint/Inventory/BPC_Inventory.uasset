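; Inventory component that stores items and amounts in a slot array and supplies ammo for weapon reloads.
; DoReload and DoesHaveAmmo match items by the weapon's ammo tag; reloading draws from the first matching stack, then another if short.
; RemoveItem decrements or clears slots, then refreshes the inventory widget through the local player controller.
; AddItemOld and CheckEmptySlot have mostly disconnected logic, and debug key 2 prints the contents.
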(event EventBeginPlay)

(event EventTick
  (params (DeltaSeconds :type Float%20%28single-precision%29)))

(event Input|KeyboardEvents|DebugKey2
  (params (Key :type Key%20Structure :default "None") (ActionValue :type Input%20Action%20Value%20Structure))
  (:Pressed
    (for _array_element (Utils|GetInventory)
      (Development|PrintString (Utilities|String|Append (Utilities|GetDisplayName (.Item (Utilities|Struct|BreakItemSlotInfo _array_element))) ": " (Utilities|String|ToString(Integer) (.AmountHeld (Utilities|Struct|BreakItemSlotInfo _array_element))))))))

(fn AddItemOld
  (params (Item :type Item%20Info%20Asset%20Object%20Reference) (Amount%20 :type Integer))
  (bind (_emptyslotindex _slotfound) (CallFunction|CheckEmptySlot))
  (if (not (Variables|/Script/ResidentSideways.ItemInfoAsset|GetbIsStackable Item))
    (if _slotfound
      (bind _output_get (LocalVariables|SetTargetSlotIndex _emptyslotindex))
      (Utilities|Array|SetArrayElem :TargetArray (Variables|Default|GetInventory) :Index _output_get)
      (return true)
      (else
        (return false)))))

(fn CheckEmptySlot)

(fn GetInventory
  (return (Variables|Default|GetInventory)))

(fn GetItematIndex
  (params (Index :type Integer))
  (return (Utilities|Array|Get(acopy) (Variables|Default|GetInventory) Index)))

(fn DoReload
  (params (RoundsInMag :type Integer) (WeaponInfo :type Item%20Info%20Asset%20Object%20Reference))
  (bind (_ammoindex _ammofound) (Ammo|CheckforBoxinSlot WeaponInfo))
  (bind (_ammoindex_2 _ammofound_2) (Ammo|CheckforBoxinSlot WeaponInfo))
  (LocalVariables|SetRoundsNeeded (- (Utilities|Struct|BreakWeaponInfo (Variables|/Script/ResidentSideways.ItemInfoAsset|GetWeaponInfo WeaponInfo)) RoundsInMag))
  (if _ammofound_2
    (LocalVariables|SetAmmoSlotIndex _ammoindex_2)
    (if (>= (Utilities|Struct|BreakItemSlotInfo (Utils|GetItematIndex (LocalVariables|GetAmmoSlotIndex))) (LocalVariables|GetRoundsNeeded))
      (CallFunction|RemoveItem (LocalVariables|GetAmmoSlotIndex) (LocalVariables|GetRoundsNeeded))
      (return (+ (LocalVariables|GetRoundsNeeded) RoundsInMag))
      (else
        (CallFunction|RemoveItem (LocalVariables|GetAmmoSlotIndex) (Utilities|Struct|BreakItemSlotInfo (Utils|GetItematIndex (LocalVariables|GetAmmoSlotIndex))))
        (if _ammofound
          (LocalVariables|SetAmmoSlotIndex _ammoindex)
          (CallFunction|RemoveItem (LocalVariables|GetAmmoSlotIndex) (LocalVariables|GetRoundsNeeded))
          (return (+ (LocalVariables|GetRoundsNeeded) RoundsInMag))
          (else
            (return (Utilities|Struct|BreakItemSlotInfo (Utils|GetItematIndex (LocalVariables|GetAmmoSlotIndex))))))))
    (else
      (return RoundsInMag))))

(fn RemoveItem
  (params (ItemIndex :type Integer) (AmountToRemove :type Integer))
  (bind _inventory (Variables|Default|GetInventory))
  (bind _inventory_2 (Variables|Default|GetInventory))
  (bind _output (Utilities|Array|Get(acopy) _inventory ItemIndex))
  (bind _output_2 (Utilities|Array|Get(acopy) _inventory_2 ItemIndex))
  (bind _returnvalue (- (.amountheld _output) AmountToRemove))
  (LocalVariables|SetFinalAmount _returnvalue)
  (if (<= _returnvalue 0)
    (Utilities|Array|SetArrayElem :TargetArray (Variables|Default|GetInventory) :Index ItemIndex)
    (else
      (Utilities|Array|SetArrayElem (Variables|Default|GetInventory) ItemIndex (Utilities|Struct|MakeItemSlotInfo (.item _output_2) (LocalVariables|GetFinalAmount) (.bslotfilled _output_2)))))
  (bind _inventorywidget (Class|BPIPlayerController|GetInventoryWidget(Message) (CallFunction|GetLocalPlayerController (Components|GetOwner))))
  (Default|UpdateInventory _inventorywidget))

(fn CheckforBoxinSlot
  (params (WeaponInfo :type Item%20Info%20Asset%20Object%20Reference))
  (bind (_array_element _array_index) (Utilities|Array|ForEachLoopwithBreak (Variables|Default|GetInventory) :!label _label)
    (:LoopBody
      (Utilities|IsValid (Utilities|Struct|BreakItemSlotInfo _array_element)
        (:Is%20Valid
          (if (== (Variables|/Script/ResidentSideways.ItemInfoAsset|GetItemTag (Utilities|Struct|BreakItemSlotInfo _array_element)) (Utilities|Struct|BreakWeaponInfo (Variables|/Script/ResidentSideways.ItemInfoAsset|GetWeaponInfo WeaponInfo)))
            (LocalVariables|SetAmmoSlotFound true)
            (LocalVariables|SetAmmoSlotIndex _array_index)
            (goto _label Break)
            (else
              _)))
        (:Is%20Not%20Valid
          _))
      (LocalVariables|SetAmmoSlotFound false))
    (:Completed
      (if (LocalVariables|GetAmmoSlotFound)
        (return (LocalVariables|GetAmmoSlotIndex) true)
        (else
          (return -1 false))))))

(fn DoesHaveAmmo
  (params (WeaponAmmoTag :type Gameplay%20Tag%20Structure))
  (for _array_element (Variables|Default|GetInventory)
    (if (.bSlotFilled (Utilities|Struct|BreakItemSlotInfo _array_element))
      (if (== (Variables|/Script/ResidentSideways.ItemInfoAsset|GetItemTag (.Item (Utilities|Struct|BreakItemSlotInfo _array_element))) WeaponAmmoTag)
        (LocalVariables|SetAmountHeld (+ (LocalVariables|GetAmountHeld) (.AmountHeld (Utilities|Struct|BreakItemSlotInfo _array_element)))))))
  (return (LocalVariables|GetAmountHeld)))