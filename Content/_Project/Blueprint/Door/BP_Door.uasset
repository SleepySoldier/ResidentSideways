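; BP_Door is an interactable door that moves the player to a linked door.
; A Box overlap with a Player-tagged actor shows the prompt Widget and sets CanInteract, and leaving hides it and clears the flag.
; OnInteract, when allowed, adds a W_Transition screen, places the interacting actor just above LinkedDoor's location and enables its input through its player controller.
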(event `self.Box.OnComponentBeginOverlap`
  (params (OverlappedComponent :type "PrimitiveComponent Object Reference") (OtherActor :type "Actor Object Reference") (OtherComp :type "PrimitiveComponent Object Reference") (OtherBodyIndex :type Integer) (bFromSweep :type Boolean) (SweepResult :type "HitResult Structure (by ref)"))
  (if (`self.ActorHasTag` OtherActor "Player")
    (`SceneComponent.SetVisibility` (`self.Widget`) true false)
    (set `self.CanInteract` true)))

(event `self.Box.OnComponentEndOverlap`
  (params (OverlappedComponent :type "PrimitiveComponent Object Reference") (OtherActor :type "Actor Object Reference") (OtherComp :type "PrimitiveComponent Object Reference") (OtherBodyIndex :type Integer))
  (if (`self.ActorHasTag` OtherActor "Player")
    (`SceneComponent.SetVisibility` (`self.Widget`) false false)
    (set `self.CanInteract` false)))

(event `/Game/_Project/Blueprint/Definitions/Interface/BPI_Interact.OnInteract`
  (params (InteractingActor :type "Actor Object Reference"))
  (if (`self.CanInteract`)
    (bind _returnvalue (`|CreateWidget` "/Game/_Project/UI/W_Transition.W_Transition_C"))
    (`UserWidget.AddToViewport` _returnvalue 0)
    (`self.K2_SetActorLocation` InteractingActor (+ (`self.K2_GetActorLocation` (`self.LinkedDoor`)) (0.0 0.0 100.0)) false false)
    (`self.EnableInput` InteractingActor (cast `PlayerController` (`Pawn.GetController` (cast `Character` InteractingActor :!pure true)) :!pure true))))

(fn `UserConstructionScript`)