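; BP_LockedDoor is an interactable door that teleports the interacting actor to its linked door, optionally requiring a key.
; A box overlap with a Player-tagged actor shows a prompt widget and sets CanInteract, which gates entry.
; OnInteract searches the inventory for an item matching the RequiredKey gameplay tag, then unlocks with a sound or shows a locked message.
; Entry happens on a later interaction once unlocked, adding a transition widget and playing a sound.
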(event `self.Box.OnComponentBeginOverlap`
  (params (OverlappedComponent :type "PrimitiveComponent Object Reference") (OtherActor :type "Actor Object Reference") (OtherComp :type "PrimitiveComponent Object Reference") (OtherBodyIndex :type Integer) (bFromSweep :type Boolean) (SweepResult :type "HitResult Structure (by ref)"))
  (if (`self.ActorHasTag` OtherActor "Player")
    (`SceneComponent.SetVisibility` (`self.Widget`) true false)
    (set `self.CanInteract` true)))

(event `self.Box.OnComponentEndOverlap`
  (params (OverlappedComponent :type "PrimitiveComponent Object Reference") (OtherActor :type "Actor Object Reference") (OtherComp :type "PrimitiveComponent Object Reference") (OtherBodyIndex :type Integer))
  (if (`self.ActorHasTag` OtherActor "Player")
    (`SceneComponent.SetVisibility` (`self.Widget`) false false)
    (set `self.CanInteract` false)))

(event `self.OnInteract`
  (params (InteractingActor :type "Actor Object Reference"))
  (set `self.Interacting Actor` InteractingActor)
  (if (`self.RequiresKey`)
    (if (`self.Unlocked`)
      (`self.EnterDoor`)
      (else
        (for _array_element (`/Game/_Project/Blueprint/Inventory/BPC_Inventory.GetInventory` (`self.GetComponentByClass` (`self.Interacting Actor`) "/Game/_Project/Blueprint/Inventory/BPC_Inventory.BPC_Inventory_C"))
          (bind ((`Item` _item)) (break `ItemSlotInfo` _array_element))
          (`/Engine/EditorBlueprintResources/StandardMacros.IsValid` _item
            (:`Is Valid`
              (if (`BlueprintGameplayTagLibrary.MatchesTag` (`ItemInfoAsset.ItemTag` _item) (`self.RequiredKey`))
                (set `self.Unlocked` true)
                (break)
                (else
                  _)))
            (:`Is Not Valid`
              _))
          (set `self.Unlocked` false))
        (if (`self.Unlocked`)
          (`GameplayStatics.PlaySound2D` (`self.UnlockDoorSound`) 1.0 1.0 0.0 null null)
          (else
            (message `/Game/_Project/Blueprint/Definitions/Interface/BPI_PlayerController.SetMessage` (`/Game/_Project/Blueprint/Definitions/FunctionLibrary/BFL_HandyTools.GetLocalPlayerController` (`self.Interacting Actor`)) "This door is locked. It looks like it needs a key.")))))
    (else
      (`self.EnterDoor`))))

(event `EnterDoor`
  (if (`self.CanInteract`)
    (bind _returnvalue (`|CreateWidget` "/Game/_Project/UI/W_Transition.W_Transition_C"))
    (`UserWidget.AddToViewport` _returnvalue 0)
    (`self.K2_SetActorLocation` (`self.Interacting Actor`) (+ (`self.K2_GetActorLocation` (`self.LinkedDoor`)) (0.0 0.0 100.0)) false false)
    (`self.EnableInput` (`self.Interacting Actor`) (`/Game/_Project/Blueprint/Definitions/FunctionLibrary/BFL_HandyTools.GetLocalPlayerController` (`self.Interacting Actor`)))
    (`GameplayStatics.PlaySound2D` (`self.EnterDoorSounds`) 1.0 1.0 0.0 null null)))

(fn `UserConstructionScript`)