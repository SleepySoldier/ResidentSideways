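; Player stats component that manages stamina for sprinting, with drain, delayed regeneration and one-off costs through UseStamina.
; StartSprint runs a fast looping timer that drains stamina and fires OnStartSprint on each step, switching to regen when stamina runs low.
; StartRegenStamina fires OnStopSprinting and starts a delayed looping refill timer that stops at max.
; Stamina changes broadcast a normalized value through OnStaminaChanged.
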(event `StartSprint`
  (`KismetSystemLibrary.K2_ClearAndInvalidateTimerHandle` (`self.RefillTimerHandle`))
  (bind _returnvalue (`KismetSystemLibrary.K2_SetTimerDelegate` (delegate `UseStam`) 0.01 true))
  (set `self.StaminaDrainTimer` _returnvalue))

(event `UseStam`
  (if (> (`self.CurrentStamina`) (`self.StaminaCost`))
    (set `self.CurrentStamina` (`KismetMathLibrary.FMax` (- (`self.CurrentStamina`) (`self.StaminaCost`))))
    (`self.BroadcastStamina`)
    (`self.OnStartSprint`)
    (else
      (`self.StartRegenStamina`))))

(event `StartRegenStamina`
  (`KismetSystemLibrary.K2_ClearAndInvalidateTimerHandle` (`self.StaminaDrainTimer`))
  (`self.StartRefillStamina`)
  (`self.OnStopSprinting`))

(event `self.ReceiveTick`
  (params (DeltaSeconds :type "Float (single-precision)")))

(event `StartRefillStamina`
  (bind _returnvalue (`KismetSystemLibrary.K2_SetTimerDelegate` (delegate `RegenStamina`) 0.01 true false (`self.RegenStartDelay`)))
  (set `self.RefillTimerHandle` _returnvalue))

(event `RegenStamina`
  (if (>= (`self.CurrentStamina`) (`self.MaxStamina`))
    (`KismetSystemLibrary.K2_ClearAndInvalidateTimerHandle` (`self.RefillTimerHandle`))
    (else
      (set `self.CurrentStamina` (`KismetMathLibrary.FMin` (+ (`self.CurrentStamina`) (`self.StaminaRegenAmount`)) (`self.MaxStamina`)))
      (`self.BroadcastStamina`))))

(fn `BroadcastStamina`
  (`self.OnStaminaChanged` (/ (`self.CurrentStamina`) (`self.MaxStamina`))))

(fn `Initialize`
  (`parent.Initialize`)
  (set `self.CurrentStamina` (`self.MaxStamina`))
  (`self.BroadcastStamina`))

(fn `RefillStamina`)

(fn `UseStamina`
  (params (DrainAmount :type "Float (double-precision)" :default 1.0))
  (set `self.CurrentStamina` (`KismetMathLibrary.FMax` (- (`self.CurrentStamina`) DrainAmount)))
  (`self.BroadcastStamina`))