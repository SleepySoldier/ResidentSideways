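; BPC_SaveGame is an actor component that saves and restores its owner's data through SidescrollGameInstance, keyed by the owner's path name.
; It loads on BeginPlay and follows the game instance's save and load events, relaying them through SaveData and LoadData dispatchers.
; SavePackageActorData passes data to the game instance for storage.
; When play ends through destruction, it removes its entry from the save map.
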(event `self.ReceiveBeginPlay`
  (bind _assidescroll_game_instance (cast `/Game/_Project/Blueprint/Game/SidescrollGameInstance` (`GameplayStatics.GetGameInstance`)))
  (set `self.GameInstance` _assidescroll_game_instance)
  (add `/Game/_Project/Blueprint/Game/SidescrollGameInstance.OnSaveGame` (`self.GameInstance`) (delegate `OnSaveGame`))
  (add `/Game/_Project/Blueprint/Game/SidescrollGameInstance.OnLoadGame` (`self.GameInstance`) (delegate `OnLoadGame`))
  (set `self.SaveID` (`KismetSystemLibrary.GetPathName` (`self.GetOwner`)))
  (`self.LoadSaveData`))

(event `OnSaveGame`
  (`self.SaveData`))

(event `OnLoadGame`
  (`self.LoadSaveData`))

(event `self.ReceiveEndPlay`
  (params (EndPlayReason :type "EEndPlayReason Enum" :default "Destroyed"))
  (switch `EEndPlayReason` EndPlayReason
    (:`Destroyed`
      (message `/Game/_Project/Blueprint/Definitions/Interface/BPI_SaveGame.RemoveFromSaveMap` (`self.GameInstance`) (`self.SaveID`)))
    (:`LevelTransition`
      _)
    (:`EndPlayInEditor`
      _)
    (:`RemovedFromWorld`
      _)
    (:`Quit`
      _))
  (set `self.GameInstance` null))

(fn `LoadSaveData`
  (if (not (`KismetStringLibrary.IsEmpty` (`self.SaveID`)))
    (bind (_valid _savedata) (message `/Game/_Project/Blueprint/Definitions/Interface/BPI_SaveGame.LoadActorData` (`self.GameInstance`) (`self.SaveID`)))
    (if _valid
      (`self.LoadData` _savedata))))

(fn `SavePackageActorData`
  (params (SaveData :type "/Game/_Project/Blueprint/Save/F_SaveData Structure"))
  (bind _output_get (set `self.SaveID` (`KismetSystemLibrary.GetPathName` (`self.GetOwner`))))
  (message `/Game/_Project/Blueprint/Definitions/Interface/BPI_SaveGame.SaveActorData` (`self.GameInstance`) _output_get SaveData))