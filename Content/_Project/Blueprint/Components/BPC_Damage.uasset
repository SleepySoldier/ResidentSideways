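; BPC_Damage is a component that tracks health, damage, healing and death.
; TakeDamage reads amount and hit response from a DamageInfo, floors health at zero, fires the hit response event, then sets IsDead and fires the death event at zero.
; Heal caps health at MaxHp, and Initialize resets it to full.
; All three broadcast health as a normalized fraction through an OnHealthChanged event.
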(event `self.ReceiveBeginPlay`)

(fn `BroadcastHealth`
  (`self.OnHealthChanged` (/ (`self.CurrentHp`) (`self.MaxHp`))))

(fn `Heal`
  (params (Amount :type "Float (double-precision)"))
  (returns (CurrentHp :type "Float (double-precision)"))
  (set `self.CurrentHp` (`KismetMathLibrary.FMin` (+ Amount (`self.CurrentHp`)) (`self.MaxHp`)))
  (`self.BroadcastHealth`)
  (return (`self.CurrentHp`)))

(fn `Initialize`
  (set `self.CurrentHp` (`self.MaxHp`))
  (`self.BroadcastHealth`))

(fn `TakeDamage`
  (params (DamageInfo :type "/Game/_Project/Blueprint/Definitions/Stuct/Damage/F_Damageinfo Structure"))
  (returns (CurrentHp :type "Float (double-precision)"))
  (set `self.CurrentHp` (`KismetMathLibrary.FMax` (- (`self.CurrentHp`) (`.Amount_2_B57285C048CEB84E8AFDA191F6B8DA3D` (break `/Game/_Project/Blueprint/Definitions/Stuct/Damage/F_Damageinfo` DamageInfo)))))
  (`self.BroadcastHealth`)
  (`self.OnHitResponse` (`.HitResponse_8_486EF0A248F13C4F93F5A3BBD9036BF0` (break `/Game/_Project/Blueprint/Definitions/Stuct/Damage/F_Damageinfo` (`local.DamageInfo`))))
  (if (<= (`self.CurrentHp`) 0.0)
    (set `self.isDead` true)
    (`self.OnDeath`)
    (return (`self.CurrentHp`))
    (else
      (return (`self.CurrentHp`)))))