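; Sidescroller game instance that manages saving and loading through an ID-keyed map of actor data, loading slot "sav1" on Init.
; Actors can add, remove or look up their entries in SaveMap.
; RequestSave broadcasts OnSaveGame, waits a frame, then writes the map to a BP_SaveGame, with an async branch and an "autosave" slot.
; Loading broadcasts OnLoadGame before restoring SaveMap from the slot.
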(event `self.ReceiveInit`
  (`self.LoadGameFromSlot` "sav1"))

(event `/Game/_Project/Blueprint/Definitions/Interface/BPI_SaveGame.SaveGameToSlot`
  (params (`Slot Name` :type String))
  (set `self.CurrentSlot` `Slot Name`)
  (`KismetSystemLibrary.PrintString` "saved to slot "))

(event `/Game/_Project/Blueprint/Definitions/Interface/BPI_SaveGame.LoadGameFromSlot`
  (params (Slot :type String))
  (set `self.CurrentSlot` Slot)
  (`self.OnLoadGame`)
  (bind _returnvalue (`GameplayStatics.DoesSaveGameExist` (`self.CurrentSlot`)))
  (if _returnvalue
    (bind _returnvalue_2 (`GameplayStatics.LoadGameFromSlot` (`self.CurrentSlot`)))
    (bind _asbp_save_game (cast `/Game/_Project/Blueprint/Save/BP_SaveGame` _returnvalue_2))
    (set `self.SaveMap` (`/Game/_Project/Blueprint/Save/BP_SaveGame.SaveMap` _asbp_save_game))))

(event `/Game/_Project/Blueprint/Definitions/Interface/BPI_SaveGame.SaveActorData`
  (params (ID :type String) (SaveData :type "/Game/_Project/Blueprint/Save/F_SaveData Structure"))
  (`BlueprintMapLibrary.Map_Add` (`self.SaveMap`) ID SaveData))

(event `/Game/_Project/Blueprint/Definitions/Interface/BPI_SaveGame.RequestSave`
  (params (Async :type Boolean) (SlotName :type String))
  (bind _output_get (set `self.Autosave` Async))
  (if _output_get
    (set `self.CurrentSlot` "autosave")
    (else
      (set `self.CurrentSlot` SlotName)))
  (`KismetSystemLibrary.PrintString` "saving...")
  (`|ExecutionSequence`
    (:`then_0`
      (`self.OnSaveGame`))
    (:`then_1`
      (`KismetSystemLibrary.DelayUntilNextFrame`)
      (bind _returnvalue (`GameplayStatics.CreateSaveGameObject` "/Game/_Project/Blueprint/Save/BP_SaveGame.BP_SaveGame_C"))
      (set `/Game/_Project/Blueprint/Save/BP_SaveGame.SaveMap` (`self.SaveMap`) _returnvalue)
      (`self.Autosave`
        (:`then`
          (`AsyncActionHandleSaveGame.AsyncSaveGameToSlot` _returnvalue (`self.CurrentSlot`)
            (:`Completed`
              _)))
        (:`else`
          (`GameplayStatics.SaveGameToSlot` _returnvalue (`self.CurrentSlot`))))
      (`KismetSystemLibrary.PrintString` "Finish saving")
      (`/Game/_Project/Blueprint/Definitions/Interface/BPI_SaveGame.SaveGameToSlot` (`self.CurrentSlot`)))))

(event `/Game/_Project/Blueprint/Definitions/Interface/BPI_SaveGame.RemoveFromSaveMap`
  (params (ID :type String))
  (`BlueprintMapLibrary.Map_Remove` (`self.SaveMap`) ID))

(fn `LoadActorData`
  (params (ID :type String))
  (returns (Valid :type Boolean) (SaveData :type "/Game/_Project/Blueprint/Save/F_SaveData Structure"))
  (bind (_value _returnvalue) (`BlueprintMapLibrary.Map_Find` (`self.SaveMap`) ID))
  (return _returnvalue _value))