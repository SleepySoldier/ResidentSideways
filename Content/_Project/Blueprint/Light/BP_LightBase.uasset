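; BP_LightBase is a proximity light that switches its RectLight on while an actor tagged Player is inside its Sphere.
; The construction script sizes the Sphere from the InSphereRadius variable, and its overlap events set the light to a fixed intensity or zero.
; On BeginPlay, a zero-length Pawn sphere trace of the same radius sets the initial state, checking only the single returned hit.
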(event `self.ReceiveBeginPlay`
  (bind _returnvalue (`self.K2_GetActorLocation`))
  (bind _outhit (`KismetSystemLibrary.SphereTraceSingleForObjects` _returnvalue _returnvalue (`SphereComponent.SphereRadius` (`self.Sphere`)) (`|MakeArray` "ObjectTypeQuery3" :!type "EObjectTypeQuery Enum")))
  (`LightComponent.SetIntensity` (`self.RectLight`) (`KismetMathLibrary.SelectFloat` 5000.0 0.0 (`self.ActorHasTag` (`.HitActor` (`GameplayStatics.BreakHitResult` _outhit)) "Player"))))

(event `self.Sphere.OnComponentBeginOverlap`
  (params (OverlappedComponent :type "PrimitiveComponent Object Reference") (OtherActor :type "Actor Object Reference") (OtherComp :type "PrimitiveComponent Object Reference") (OtherBodyIndex :type Integer) (bFromSweep :type Boolean) (SweepResult :type "HitResult Structure (by ref)"))
  (if (`self.ActorHasTag` OtherActor "Player")
    (`LightComponent.SetIntensity` (`self.RectLight`) 5000.0)))

(event `self.Sphere.OnComponentEndOverlap`
  (params (OverlappedComponent :type "PrimitiveComponent Object Reference") (OtherActor :type "Actor Object Reference") (OtherComp :type "PrimitiveComponent Object Reference") (OtherBodyIndex :type Integer))
  (if (`self.ActorHasTag` OtherActor "Player")
    (`LightComponent.SetIntensity` (`self.RectLight`) 0.0)))

(fn `UserConstructionScript`
  (`SphereComponent.SetSphereRadius` (`self.Sphere`) (`self.In Sphere Radius`) true))