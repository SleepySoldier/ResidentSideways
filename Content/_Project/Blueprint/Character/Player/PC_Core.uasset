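; PC_Core is the player controller that manages input mapping and the player's UI, from title menu to in-game HUD and inventory.
; It adds the default Enhanced Input context on BeginPlay, and the menu input opens the inventory with UI-only input and a cursor.
; Separate events show the title screen or build the HUD and inventory widgets, then initialize the pawn's player stats component.
; It also relays messages to the HUD and exposes the inventory widget.
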(event `self.ReceiveBeginPlay`
  ;[1 1 1] Add regular input mappings
  (`EnhancedInputSubsystemInterface.AddMappingContext` (subsystem `EnhancedInputLocalPlayerSubsystem`) "/Game/_Project/Input/IMC_Default.IMC_Default" 0 (struct)))

(event `EnhancedInput|/Game/_Project/Input/Actions/IA_OpenMenu`
  (params (ActionValue :type Boolean) (ElapsedSeconds :type "Float (double-precision)") (TriggeredSeconds :type "Float (double-precision)") (InputAction :type "InputAction Object Reference" :default "/Game/_Project/Input/Actions/IA_OpenMenu.IA_OpenMenu"))
  (:`Started`
    (if (not (`Widget.IsInViewport` (`self.InventoryWidget`)))
      (`UserWidget.AddToViewport` (`self.InventoryWidget`) 0)
      (`WidgetBlueprintLibrary.SetInputMode_UIOnlyEx` self (`self.InventoryWidget`) "DoNotLock" true)
      (set `self.bShowMouseCursor` true))))

(event `/Game/_Project/Blueprint/Definitions/Interface/BPI_PlayerController.SetMessage`
  (params (Message :type String))
  (`/Game/_Project/UI/W_MainUILayout.DisplayMessage` (`self.MainHud`) Message))

(event `/Game/_Project/Blueprint/Definitions/Interface/BPI_PlayerController.InitializePlayerOverlay`
  (bind _returnvalue (`|CreateWidget` "/Game/_Project/UI/W_MainUILayout.W_MainUILayout_C" self))
  (bind _output_get (set `self.MainHud` _returnvalue))
  (`UserWidget.AddToViewport` _output_get 0)
  (bind _returnvalue_2 (`|CreateWidget` "/Game/_Project/UI/Inventory/W_MainInventory.W_MainInventory_C" self))
  (set `self.InventoryWidget` _returnvalue_2)
  (`/Game/_Project/Blueprint/Components/BPC_Damage.Initialize` (`self.GetComponentByClass` (`self.K2_GetPawn`) "/Game/_Project/Blueprint/Components/BPC_PlayerStats.BPC_PlayerStats_C"))
  (`WidgetBlueprintLibrary.SetInputMode_GameOnly` self true)
  (set `self.bShowMouseCursor` false))

(event `/Game/_Project/Blueprint/Definitions/Interface/BPI_PlayerController.InitTitleMenu`
  (bind _returnvalue (`|CreateWidget` "/Game/_Project/UI/W_Title.W_Title_C" self))
  (`UserWidget.AddToViewport` _returnvalue 0)
  (set `self.bShowMouseCursor` true)
  (`WidgetBlueprintLibrary.SetInputMode_UIOnlyEx` self _returnvalue "DoNotLock" true))

(fn `GetInventoryWidget`
  (returns (InventoryWidget :type "/Game/_Project/UI/Inventory/W_MainInventory Object Reference"))
  (return (`self.InventoryWidget`)))

(fn `UserConstructionScript`)