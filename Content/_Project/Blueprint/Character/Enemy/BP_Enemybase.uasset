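; Base enemy character that exposes behavior tree, patrol route, attack and health data through getters.
; BPC_Damage handles health, driving chance-based hit reacts and a death that stops AI logic and ragdolls on montage blend-out.
; Attack requests select default, run, random-section or grab montages; the grab sphere-traces for the player, snaps into place and plays paired montages.
; Incoming damage spawns impact effects and reports a damage sense event.
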(event `self.ReceiveBeginPlay`
  (`/Game/_Project/Blueprint/Components/BPC_Damage.Initialize` (`self.BPC_Damage`)))

(event `self.BPC_Damage.OnHitResponse`
  (params (HitResponse :type "/Game/_Project/Blueprint/Definitions/Enumerator/Damage/E_HitResponse Enum" :default "NewEnumerator0"))
  (switch `/Game/_Project/Blueprint/Definitions/Enumerator/Damage/E_HitResponse` HitResponse
    (:`NewEnumerator1`
      (if (`KismetMathLibrary.RandomBoolWithWeight` (`self.HitReactChance`))
        (`|PlayMontage` (`self.Mesh`) (`self.HitReactMontage`))))))

(event `self.BPC_Damage.OnDeath`
  (bind _mesh (`self.Mesh`))
  (`BrainComponent.StopLogic` (`AIController.BrainComponent` (`AIBlueprintHelperLibrary.GetAIController` self)) "Dead")
  (set `PrimitiveComponent.bGenerateOverlapEvents` false (`self.Mesh`))
  (`PrimitiveComponent.SetCollisionEnabled` (`self.CapsuleComponent`) "NoCollision")
  (`|PlayMontage` (`self.Mesh`) (`self.DeathMontage`)
    (:`OnBlendOut`
      (`PrimitiveComponent.SetCollisionEnabled` _mesh "PhysicsOnly")
      (`PrimitiveComponent.SetCollisionResponseToChannel` _mesh "ECC_GameTraceChannel2" "ECR_Block")
      (`PrimitiveComponent.SetSimulatePhysics` _mesh true))))

(event `ImpactFX`
  (params (DamageInfo :type "/Game/_Project/Blueprint/Definitions/Stuct/Damage/F_Damageinfo Structure"))
  (bind ((`HitLocation_5_32A0328C4B177BB61D12B0BC7B470489` _hitlocation)) (break `/Game/_Project/Blueprint/Definitions/Stuct/Damage/F_Damageinfo` DamageInfo))
  ;[0 0 0 0.5] Effects on impact
  (`NiagaraFunctionLibrary.SpawnSystemAtLocation` (`self.MeleeImpactSystem`) _hitlocation)
  (`GameplayStatics.PlayWorldCameraShake` "/Game/_Project/Blueprint/Camera/CS_ImpactShake.CS_ImpactShake_C" _hitlocation 0.0 2000.0 0.0 true)
  (`GameplayStatics.PlaySoundAtLocation` "/Game/_Project/Effects/Sound/MetaSound/SFX_ShotgunBodyImpact.SFX_ShotgunBodyImpact" _hitlocation (struct) 1.0 0.6 0.0 null null null null))

(event `/Game/_Project/Blueprint/Definitions/Interface/BPI_EnemyAI.SetWalkSpeed`
  (params (WalkSpeed :type "/Game/_Project/Blueprint/Character/Enemy/AI/E_Gait Enum" :default "NewEnumerator0"))
  ;[0 0 0 0.5] Set max walk speed form Enemy AI
  (`self.SetMaxWalkSpeed` (select `/Game/_Project/Blueprint/Character/Enemy/AI/E_Gait` WalkSpeed :`NewEnumerator1` (`self.WalkSpeed`) :`NewEnumerator2` (`self.RunSpeed`) :`NewEnumerator3` (`self.CrawlSpeed`) :!type "Float (single-precision)")))

(event `Attack`
  (params (Attacks :type "/Game/_Project/Blueprint/Character/Enemy/AI/E_EnemyAttacks Enum" :default "NewEnumerator0"))
  ;[0 0 0 0.5] Attacks
  (switch `/Game/_Project/Blueprint/Character/Enemy/AI/E_EnemyAttacks` Attacks
    (:`NewEnumerator0`
      (`self.DefaultAttack`))
    (:`NewEnumerator1`
      (`self.GrabAttack`))
    (:`NewEnumerator2`
      (`self.RunAttack`))
    (:`NewEnumerator3`
      (`self.RandomAttack`))))

(event `GrabAttack`
  (bind _returnvalue (`self.K2_GetActorLocation`))
  ;[0 0 0 0.5] Attacks
  ;;[0 0 0 0.5] Grab Attack
  (bind _outhit (`KismetSystemLibrary.SphereTraceSingleForObjects` :`Start` _returnvalue :`End` (+ _returnvalue (* (`self.GetActorForwardVector`) 100.0)) :`Radius` 30.0 :`ObjectTypes` (`|MakeArray` "ObjectTypeQuery8" :!type "EObjectTypeQuery Enum") :`DrawDebugType` "ForDuration"))
  (bind (_bblockinghit _binitialoverlap _time _distance _location _impactpoint _normal _impactnormal _physmat _hitactor) (`GameplayStatics.BreakHitResult` _outhit))
  (if (`self.ActorHasTag` _hitactor "Player")
    (`|ExecutionSequence`
      (:`then_0`
        (bind _playercontroller (`/Game/_Project/Blueprint/Definitions/FunctionLibrary/BFL_HandyTools.GetLocalPlayerController` _hitactor))
        (`self.DisableInput` _hitactor _playercontroller)
        (`Controller.SetIgnoreMoveInput` _playercontroller false)
        (`PrimitiveComponent.SetCollisionEnabled` (`self.CapsuleComponent`) "NoCollision")
        (bind _returnvalue_2 (`self.K2_GetActorLocation` _hitactor))
        (`self.K2_SetActorLocation` (+ _returnvalue_2 (* (`self.GetActorForwardVector` _hitactor) 10.0)))
        (`self.K2_SetActorRotation` (`KismetMathLibrary.FindLookAtRotation` (`self.K2_GetActorLocation`) _returnvalue_2)))
      (:`then_1`
        (`|PlayMontage` (`self.GetComponentByClass` _hitactor "/Script/Engine.SkeletalMeshComponent") (`self.GrabVicMontage`)
          (:`then`
            (bind _notifyname (`|PlayMontage` (`self.Mesh`) (`self.GrabAtkMontage`))
              (:`OnCompleted`
                (`PrimitiveComponent.SetCollisionEnabled` (`self.CapsuleComponent`) "QueryAndPhysics")
                (`self.OnAttackEnd` :!label _label)
                (`self.EnableInput` _hitactor (`/Game/_Project/Blueprint/Definitions/FunctionLibrary/BFL_HandyTools.GetLocalPlayerController` _hitactor))
                (`self.EnableInput` _hitactor (`/Game/_Project/Blueprint/Definitions/FunctionLibrary/BFL_HandyTools.GetLocalPlayerController` _hitactor)))
              (:`OnInterrupted`
                (goto _label))
              (:`OnNotifyBegin`
                (switch `name` _notifyname
                  (:`Damage`
                    (message `/Game/_Project/Blueprint/Definitions/Interface/BPI_Damage.TakeDamage` _hitactor (make `/Game/_Project/Blueprint/Definitions/Stuct/Damage/F_Damageinfo` (`self.Attack Damage`) _location "NewEnumerator0" self))))))))))
    (else
      (`self.OnAttackEnd`))))

(event `DefaultAttack`
  ;[0 0 0 0.5] Attacks
  ;;[0 0 0 0.5] DefaultAttack
  (`|PlayMontage` (`self.Mesh`) (`self.DefaultAttackMontage`)
    (:`OnCompleted`
      _)
    (:`OnInterrupted`
      _))
  (`self.OnAttackEnd`))

(event `RandomAttack`
  ;[0 0 0 0.5] Attacks
  ;;[0 0 0 0.5] Random Attack
  (`|PlayMontage` (`self.Mesh`) (`self.RandomAttackMontage`) 1.0 0.0 (`/Game/_Project/Blueprint/Definitions/FunctionLibrary/BFL_HandyTools.GetRandomMontageSection` (`self.RandomAttackMontage`))
    (:`OnCompleted`
      _)
    (:`OnInterrupted`
      _))
  (`self.OnAttackEnd`))

(event `RunAttack`
  ;[0 0 0 0.5] Attacks
  ;;[0 0 0 0.5] Run Attack
  (`|PlayMontage` (`self.Mesh`) (`self.RunAttackMontage`)
    (:`OnCompleted`
      _)
    (:`OnInterrupted`
      _))
  (`self.OnAttackEnd`))

(fn `GetAttackDamage`
  (returns (AttackDamage :type "Float (double-precision)") (HitResponse :type "/Game/_Project/Blueprint/Definitions/Enumerator/Damage/E_HitResponse Enum"))
  (return (`self.Attack Damage`) "NewEnumerator1"))

(fn `GetAttackRadius`
  (returns (AttackRadius :type "Float (double-precision)") (GrabAttackRadius :type "Float (double-precision)"))
  (return (`self.Attack Radius`) (`self.Grab Attack Radius`)))

(fn `GetBehaviorTree`
  (returns (ReturnValue :type "BehaviorTree Object Reference"))
  (return (`self.BehaviorTree`)))

(fn `GetCurrentHp`
  (returns (CurrentHp :type "Float (double-precision)"))
  (return (`/Game/_Project/Blueprint/Components/BPC_Damage.CurrentHp` (`self.BPC_Damage`))))

(fn `GetMaxHp`
  (returns (MaxHp :type "Float (double-precision)"))
  (return (`/Game/_Project/Blueprint/Components/BPC_Damage.MaxHp` (`self.BPC_Damage`))))

(fn `GetPatrolRoute`
  (returns (ReturnValue :type "/Game/_Project/Blueprint/Character/Enemy/AI/BP_PatrolRoute Object Reference"))
  (return (`self.PatrolRoute`)))

(fn `GetWeaponSocketLocation`
  (returns (WeaponStart :type "Vector Structure") (WeaponEnd :type "Vector Structure"))
  (return (0.0 0.0 0.0) (0.0 0.0 0.0)))

(fn `Heal`
  (params (Amount :type "Float (double-precision)"))
  (returns (Health :type "Float (double-precision)"))
  (bind _currenthp (`/Game/_Project/Blueprint/Components/BPC_Damage.Heal` (`self.BPC_Damage`) Amount))
  (return _currenthp))

(fn `IsDead`
  (returns (ReturnValue :type Boolean))
  (return (`/Game/_Project/Blueprint/Components/BPC_Damage.isDead` (`self.BPC_Damage`))))

(fn `SetMaxWalkSpeed`
  (params (`Max Walk Speed` :type "Float (single-precision)"))
  (set `CharacterMovementComponent.MaxWalkSpeed` `Max Walk Speed` (`self.CharacterMovement`)))

(fn `TakeDamage`
  (params (HitInfo :type "/Game/_Project/Blueprint/Definitions/Stuct/Damage/F_Damageinfo Structure"))
  (returns (Health :type "Float (double-precision)"))
  (bind ((`Amount_2_B57285C048CEB84E8AFDA191F6B8DA3D` _amount) (`HitLocation_5_32A0328C4B177BB61D12B0BC7B470489` _hitlocation) (`HitInstigator_11_7F984E6145FCAC509D5987BB445ED6F3` _hitinstigator)) (break `/Game/_Project/Blueprint/Definitions/Stuct/Damage/F_Damageinfo` (`local.HitInfo`)))
  (`self.ImpactFX` HitInfo)
  (bind _currenthp (`/Game/_Project/Blueprint/Components/BPC_Damage.TakeDamage` (`self.BPC_Damage`) HitInfo))
  (`AISense_Damage.ReportDamageEvent` self _hitinstigator _amount _hitlocation)
  (return _currenthp))

(fn `UserConstructionScript`)