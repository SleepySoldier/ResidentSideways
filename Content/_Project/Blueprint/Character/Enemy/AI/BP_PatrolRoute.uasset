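; BP_PatrolRoute is a spline-based patrol route actor for enemy AI.
; It tracks a current point index and returns that spline point's world location through GetLocationAtPoint.
; IncrementSplinePoint steps the index by a direction value, which flips at the last and first points so the route is traversed back and forth rather than looped.
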(event `IncrementSplinePoint`
  (set `self.Point Index` (+ (`self.Point Index`) (`self.Direction`)))
  (if (== (`self.Point Index`) (- (`SplineComponent.GetNumberOfSplinePoints` (`self.Spline`)) 1))
    (set `self.Direction` -1)
    (elif (== (`self.Point Index`) 0)
      (set `self.Direction` 1))))

(fn `GetLocationAtPoint`
  (returns (ReturnValue :type "Vector Structure"))
  (return (`SplineComponent.GetLocationAtSplinePoint` (`self.Spline`) (`self.Point Index`) "World")))

(fn `UserConstructionScript`)